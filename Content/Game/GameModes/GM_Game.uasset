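; GM_Game is the game mode that owns the rhythm and leveling managers and picks each player's start point.
; It spawns BP_BeatManager on BeginPlay, while BP_XpManager spawns lazily; both getters create their manager if missing, then return the cached instance.
; ChoosePlayerStart offers the player controller to each PST_Base actor and returns the first that accepts the spawn request.
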(event `self.ReceiveBeginPlay`
  (`parent.ReceiveBeginPlay`)
  (`self.Spawn Rhythym`))

(event `Spawn Rhythym`
  (`/Engine/EditorBlueprintResources/StandardMacros.IsValid` (`self.Beat Manager`)
    (:`Is Not Valid`
      (bind _returnvalue (`|SpawnActorFromClass` "/Game/MartinsCoolerContentFolder/BP_BeatManager.BP_BeatManager_C" (`KismetMathLibrary.MakeTransform` (0.0 0.0 0.0)) "Undefined" "MultiplyWithRoot" null null))
      (set `self.Beat Manager` _returnvalue))))

(event `Spawn LEveling`
  (`/Engine/EditorBlueprintResources/StandardMacros.IsValid` (`self.Xp Manager`)
    (:`Is Not Valid`
      (bind _returnvalue (`|SpawnActorFromClass` "/Game/Game/GameModes/BP_XpManager.BP_XpManager_C" (`KismetMathLibrary.MakeTransform` (0.0 0.0 0.0)) "Undefined" "MultiplyWithRoot" null null))
      (set `self.Xp Manager` _returnvalue))))

(fn `ChoosePlayerStart`
  (params (Player :type "Controller Object Reference"))
  (returns (ReturnValue :type "Actor Object Reference"))
  (bind _asplayer_controller (cast `PlayerController` Player))
  (bind _outactors (`GameplayStatics.GetAllActorsOfClass` "/Game/Game/PlayerStarts/PST_Base.PST_Base_C"))
  (for _array_element _outactors
    (bind _succesful (`/Game/Game/PlayerStarts/PST_Base.Request Player Spawn` _array_element _asplayer_controller))
    (if _succesful
      (return _array_element))))

(fn `Get Leveling Manager`
  (returns (ReturnValue :type "/Game/Game/GameModes/BP_XpManager Object Reference"))
  (bind _xp_manager (`self.Xp Manager`))
  (`/Engine/EditorBlueprintResources/StandardMacros.IsValid` _xp_manager
    (:`Is Valid`
      (return _xp_manager))
    (:`Is Not Valid`
      (`self.Spawn LEveling`)
      (return (`self.Xp Manager`)))))

(fn `Get Rhythym Manager`
  (returns (ReturnValue :type "/Game/MartinsCoolerContentFolder/BP_BeatManager Object Reference"))
  (bind _beat_manager (`self.Beat Manager`))
  (`/Engine/EditorBlueprintResources/StandardMacros.IsValid` _beat_manager
    (:`Is Valid`
      (return _beat_manager))
    (:`Is Not Valid`
      (`self.Spawn Rhythym`)
      (return (`self.Beat Manager`)))))

(fn `UserConstructionScript`
  (`parent.UserConstructionScript`))