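; BP_XpManager is an actor that tracks XP and level progression.
; AddXp adds an amount to XP and calls the GainedXP event dispatcher with the gain, previous value and new total.
; When XP reaches a threshold that scales linearly with the current level, it resets XP to zero, discarding overflow, increments Level once and calls LeveledUp with the old and new levels.
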(event `Add Xp`
  (params (Amount :type Integer))
  (bind _output_get (set `self.XP` (+ (`self.XP`) Amount)))
  (`self.Gained XP` Amount (- _output_get Amount) _output_get)
  (if (>= (`self.XP`) (* (`self.Level`) 100))
    (set `self.XP` 0)
    (bind _output_get_2 (set `self.Level` (+ (`self.Level`) 1)))
    (`self.Leveled Up` (- _output_get_2 1) _output_get_2)))

(fn `UserConstructionScript`)