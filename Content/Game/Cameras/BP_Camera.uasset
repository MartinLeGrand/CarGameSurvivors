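; BP_Camera is a shared camera actor that follows up to two players.
; Each tick it teleports to the midpoint of player pawns 0 and 1, or onto pawn 0 when pawn 1 is invalid.
; The spring arm length zooms between MinLength and MaxLength using the pawns' separation plus a fixed offset, clamped to that range, and stays at MinLength with one player.
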(event `self.ReceiveTick`
  (params (DeltaSeconds :type "Float (single-precision)"))
  (bind _returnvalue (`GameplayStatics.GetPlayerPawn` 1))
  (bind _returnvalue_2 (`self.K2_GetActorLocation` (`GameplayStatics.GetPlayerPawn` 0)))
  (`|ExecutionSequence`
    (:`then_0`
      (`/Engine/EditorBlueprintResources/StandardMacros.IsValid` _returnvalue
        (:`Is Valid`
          (`self.K2_SetActorLocation` (* (+ (`self.K2_GetActorLocation` _returnvalue) _returnvalue_2) 0.5) false true))
        (:`Is Not Valid`
          (`self.K2_SetActorLocation` _returnvalue_2 false true))))
    (:`then_1`
      (`/Engine/EditorBlueprintResources/StandardMacros.IsValid` (`GameplayStatics.GetPlayerPawn` 1)
        (:`Is Valid`
          (set `SpringArmComponent.TargetArmLength` (`KismetMathLibrary.Lerp` (`self.Min Length`) (`self.Max Length`) (`KismetMathLibrary.FClamp` (/ (- (+ (`self.GetDistanceTo` (`GameplayStatics.GetPlayerPawn` 0) (`GameplayStatics.GetPlayerPawn` 1)) 2500.0) (`self.Min Length`)) (- (`self.Max Length`) (`self.Min Length`))))) (`self.SpringArm`)))
        (:`Is Not Valid`
          (set `SpringArmComponent.TargetArmLength` (`self.Min Length`) (`self.SpringArm`)))))))

(fn `UserConstructionScript`)