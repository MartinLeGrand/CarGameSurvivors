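; Base enemy that chases the nearer of up to two player cars, damages players on overlap and awards XP on death.
; Staggered timers refresh the target and a separation nudge from nearby enemies, which steers the swept, horizontal movement each tick.
; Its cube billboards toward player 0's camera, with timelines driving material hurt flashes and a shrinking death effect.
; Health getters are stubs returning zero, while Targetable turns off when dying.
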(event `self.ReceiveTick`
  (params (DeltaSeconds :type "Float (single-precision)"))
  (`self.AlignToCamera`)
  (`self.MoveToPlayer`))

(event `MoveToPlayer`
  (bind (_returnvalue_x _returnvalue_y) (`KismetMathLibrary.BreakVector` (`self.K2_GetActorLocation`)))
  (bind (_returnvalue_x_2 _returnvalue_y_2) (`KismetMathLibrary.BreakVector` (`self.K2_GetActorLocation` (`self.Closest Player`))))
  (`self.K2_SetActorLocation` (+ (`self.K2_GetActorLocation`) (* (`KismetMathLibrary.Normal` (+ (`KismetMathLibrary.Normal` (- (`KismetMathLibrary.MakeVector` _returnvalue_x_2 _returnvalue_y_2) (`KismetMathLibrary.MakeVector` _returnvalue_x _returnvalue_y))) (* (`self.FinalNudgeVector`) (`self.NudgeStrength`)))) (`self.Speed`) (`GameplayStatics.GetWorldDeltaSeconds`))) true))

(event `self.ReceiveBeginPlay`
  (`self.GetTargetCar`)
  (bind _returnvalue (`KismetMaterialLibrary.CreateDynamicMaterialInstance` (`PrimitiveComponent.GetMaterial` (`self.Cube`) 0)))
  (bind _output_get (set `self.Material` _returnvalue))
  (`PrimitiveComponent.SetMaterial` (`self.Cube`) 0 _output_get)
  (`|ExecutionSequence`
    (:`then_0`
      (`KismetSystemLibrary.K2_SetTimerDelegate` (delegate `GetTargetCar`) 1.0 true false (`KismetMathLibrary.RandomFloat`)))
    (:`then_1`
      (`KismetSystemLibrary.K2_SetTimerDelegate` (delegate `Nudge`) 0.1 true false (/ (`KismetMathLibrary.RandomFloat`) 10.0)))))

(event `GetTargetCar`
  (bind _closestplayer (`self.GetClosestCar`))
  (if (not (== _closestplayer (`self.Closest Player`)))
    (set `self.Closest Player` _closestplayer)))

(event `AlignToCamera`
  (bind (_returnvalue_roll _returnvalue_pitch _returnvalue_yaw) (`KismetMathLibrary.BreakRotator` (`KismetMathLibrary.FindLookAtRotation` (`SceneComponent.K2_GetComponentLocation` (`self.Cube`)) (`PlayerCameraManager.GetCameraLocation` (`GameplayStatics.GetPlayerCameraManager` 0)))))
  (`SceneComponent.K2_SetWorldRotation` (`self.Cube`) (`KismetMathLibrary.MakeRotator` (+ _returnvalue_roll 45.0) 0.0 (+ _returnvalue_yaw -90.0)) false true))

(event `Nudge`
  (`self.CalculateNudge`))

(event `Hurt`
  (bind (_direction _multiplier) (`Timeline|HurtTimeline` :!via `PlayFromStart`)
    (:`Update`
      (`MaterialInstanceDynamic.SetScalarParameterValue` (`self.Material`) "Hurt" _multiplier))))

(event `/Game/Game/Pawns/IF_Health.Damage`
  (params (Amount :type Integer))
  (bind _output_get (set `self.Health` (- (`self.Health`) Amount)))
  (if (<= _output_get 0)
    (`self.Die`)
    (else
      (`self.Hurt`))))

(event `Die`
  (if (not (`self.Dying`))
    (`self.Hurt`)
    (set `self.Dying` true)
    (set `self.TargetableBool` false)
    (bind (_direction _multiplier) (`Timeline|Timeline` :!via `PlayFromStart`)
      (:`Update`
        (`MaterialInstanceDynamic.SetScalarParameterValue` (`self.Material`) "Kill" _multiplier)
        (`self.SetActorScale3D` (* (1.0 1.0 1.0) (- 1.0 _multiplier))))
      (:`Finished`
        (`/Game/Game/GameModes/BP_XpManager.Add Xp` (`/Game/Game/GameModes/Getters.Get XP Manager`) (`self.EXP On Death`))
        (`self.K2_DestroyActor`)))))

(event `self.Sphere.OnComponentBeginOverlap`
  (params (OverlappedComponent :type "PrimitiveComponent Object Reference") (OtherActor :type "Actor Object Reference") (OtherComp :type "PrimitiveComponent Object Reference") (OtherBodyIndex :type Integer) (bFromSweep :type Boolean) (SweepResult :type "HitResult Structure (by ref)"))
  (bind _returnvalue (`self.ActorHasTag` OtherActor "Player"))
  (`KismetSystemLibrary.PrintString` (`KismetSystemLibrary.GetDisplayName` OtherActor))
  (`KismetSystemLibrary.PrintString` (`KismetStringLibrary.Conv_BoolToString` _returnvalue))
  (if _returnvalue
    (message `/Game/Game/Pawns/IF_Health.Damage` OtherActor (`self.DamageAmount`))))

(fn `CalculateNudge`
  (locals (TotalNudgeVector :type "Vector Structure"))
  (bind (_returnvalue_x _returnvalue_y) (`KismetMathLibrary.BreakVector` (`self.K2_GetActorLocation`)))
  (bind _outactors (`KismetSystemLibrary.SphereOverlapActors` (`self.K2_GetActorLocation`) (`self.EnemySizeRadius`) (`|MakeArray` "ObjectTypeQuery3" :!type "EObjectTypeQuery Enum") "/Script/Engine.Actor" (`|MakeArray` self :!type "Actor Object Reference")))
  (for _array_element _outactors
    (if (`self.ActorHasTag` _array_element "Enemy")
      (bind (_returnvalue_x_2 _returnvalue_y_2) (`KismetMathLibrary.BreakVector` (`self.K2_GetActorLocation` _array_element)))
      (set `local.TotalNudgeVector` (+ (`KismetMathLibrary.Normal` (- (`KismetMathLibrary.MakeVector` _returnvalue_x _returnvalue_y) (`KismetMathLibrary.MakeVector` _returnvalue_x_2 _returnvalue_y_2))) (`local.TotalNudgeVector`)))))
  (set `self.FinalNudgeVector` (`local.TotalNudgeVector`)))

(fn `Get Current Health`
  (returns (ReturnValue :type Integer))
  (return 0))

(fn `Get Current Health Percent`
  (returns (ReturnValue :type "Float (double-precision)"))
  (return 0.0))

(fn `GetClosestCar`
  (returns (ClosestPlayer :type "Pawn Object Reference"))
  (`/Engine/EditorBlueprintResources/StandardMacros.IsValid` (`GameplayStatics.GetPlayerPawn` 1)
    (:`Is Valid`
      (if (> (`self.GetSquaredHorizontalDistanceTo` (`GameplayStatics.GetPlayerPawn` 0)) (`self.GetSquaredHorizontalDistanceTo` (`GameplayStatics.GetPlayerPawn` 1)))
        (return (`GameplayStatics.GetPlayerPawn` 1))
        (else
          (return (`GameplayStatics.GetPlayerPawn` 0)))))
    (:`Is Not Valid`
      (return (`GameplayStatics.GetPlayerPawn` 0)))))

(fn `Targetable`
  (returns (Targetable :type Boolean))
  (return (`self.TargetableBool`)))

(fn `UserConstructionScript`)