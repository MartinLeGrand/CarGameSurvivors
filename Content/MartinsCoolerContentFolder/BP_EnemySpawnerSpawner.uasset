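; Manager actor that repopulates the world with enemy spawners on each XP level-up, with an initial level-one trigger shortly after BeginPlay.
; Each level-up destroys existing BP_EnemySpawner actors, then spawns a per-level count from SpawnersToSpawn, passing in the new level.
; Spawners land at random points in a rectangle around the world origin.
; It also toggles boss-spawned and boss-dead FMOD music parameters through the Beat Manager at specific levels.
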(event `self.ReceiveBeginPlay`
  (add `/Game/Game/GameModes/BP_XpManager.Leveled Up` (`/Game/Game/GameModes/Getters.Get XP Manager`) (delegate `Leveled Up_Event`))
  (`KismetSystemLibrary.Delay` 1.0)
  (`self.Leveled Up_Event` 0 1))

(event `Leveled Up_Event`
  (params (`Previous Level` :type Integer) (`New Level` :type Integer))
  (bind _output_get (set `self.New Level` `New Level`))
  (bind _outactors (`GameplayStatics.GetAllActorsOfClass` "/Game/MartinsCoolerContentFolder/BP_EnemySpawner.BP_EnemySpawner_C"))
  (for _array_element _outactors
    (`self.K2_DestroyActor` _array_element))
  (for _ (range 1 (+ (`|GetArrayItem` (`self.SpawnersToSpawn`) _output_get) 1))
    (`KismetSystemLibrary.PrintString` "Spawning Spawner")
    (`self.SpawnSpawner`))
  (`|ExecutionSequence`
    (:`then_0`
      (if (== (`self.New Level`) 10)
        (`FMODAudioComponent.SetParameter` (`/Game/MartinsCoolerContentFolder/BP_BeatManager.FMODAudio` (`/Game/Game/GameModes/Getters.Get Beat Manager`)) "bossDead" 1.0)
        (else
          (`FMODAudioComponent.SetParameter` (`/Game/MartinsCoolerContentFolder/BP_BeatManager.FMODAudio` (`/Game/Game/GameModes/Getters.Get Beat Manager`)) "bossDead" 0.0))))
    (:`then_1`
      (if (== (`self.New Level`) 9)
        (`FMODAudioComponent.SetParameter` (`/Game/MartinsCoolerContentFolder/BP_BeatManager.FMODAudio` (`/Game/Game/GameModes/Getters.Get Beat Manager`)) "bossSpawned" 1.0)
        (else
          (`FMODAudioComponent.SetParameter` (`/Game/MartinsCoolerContentFolder/BP_BeatManager.FMODAudio` (`/Game/Game/GameModes/Getters.Get Beat Manager`)) "bossSpawned" 0.0))))))

(event `SpawnSpawner`
  (bind _returnvalue (`KismetMathLibrary.RandomFloatInRange` 0.0 100.0))
  (bind _returnvalue_2 (`KismetMathLibrary.RandomFloatInRange` 0.0 50.0))
  (`|SpawnActorFromClass` "/Game/MartinsCoolerContentFolder/BP_EnemySpawner.BP_EnemySpawner_C" (`KismetMathLibrary.MakeTransform` (* (`KismetMathLibrary.MakeVector` (`KismetMathLibrary.SelectFloat` _returnvalue_2 (* _returnvalue_2 -1.0) (`KismetMathLibrary.RandomBool`)) (`KismetMathLibrary.SelectFloat` _returnvalue (* _returnvalue -1.0) (`KismetMathLibrary.RandomBool`))) 100.0)) "Undefined" "MultiplyWithRoot" null (`self.New Level`) null))

(fn `UserConstructionScript`)