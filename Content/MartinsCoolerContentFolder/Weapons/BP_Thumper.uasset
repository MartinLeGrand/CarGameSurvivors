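; BP_Thumper is a car weapon that damages enemies in an area on the ground around the car when triggered.
; TriggerWeapon runs the parent logic, then traces straight down from the car and spawns an actor at the hit location.
; A sphere overlap there finds BP_EnemyBase pawns, and those tagged Enemy that report as targetable receive WeaponDamage through DamageMessage.
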(event `self.ReceiveTick`
  (params (DeltaSeconds :type "Float (single-precision)"))
  (`parent.ReceiveTick` DeltaSeconds))

(fn `TriggerWeapon`
  (bind _returnvalue (`self.K2_GetActorLocation` (`self.Car`)))
  (`parent.TriggerWeapon`)
  (bind _outhit (`KismetSystemLibrary.LineTraceSingle` _returnvalue (- _returnvalue (0.0 0.0 1000.0)) "TraceTypeQuery1" false (`|MakeArray` (`self.Car`) :!type "Actor Object Reference")))
  (bind (_bblockinghit _binitialoverlap _time _distance _location) (`GameplayStatics.BreakHitResult` _outhit))
  (`|SpawnActorFromClass` "/Game/MartinsCoolerContentFolder/Weapons/Thumper/BP_ThumperProjectile.BP_ThumperProjectile_C" (`KismetMathLibrary.MakeTransform` _location) "Undefined" "MultiplyWithRoot" null null)
  (bind (_outactors _returnvalue_2) (`KismetSystemLibrary.SphereOverlapActors` _location 1000.0 (`|MakeArray` "ObjectTypeQuery3" :!type "EObjectTypeQuery Enum") "/Game/MartinsCoolerContentFolder/BP_EnemyBase.BP_EnemyBase_C" (`|MakeArray` self)))
  (if _returnvalue_2
    (for _array_element _outactors
      (if (`self.ActorHasTag` _array_element "Enemy")
        (bind _targetable (message `/Game/MartinsCoolerContentFolder/I_Targetable.Targetable` _array_element))
        (if _targetable
          (message `/Game/Game/Pawns/IF_Health.Damage` _array_element (`self.WeaponDamage`)))))))

(fn `UserConstructionScript`
  (`parent.UserConstructionScript`))