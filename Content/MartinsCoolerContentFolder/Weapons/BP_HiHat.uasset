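; BP_HiHat is a car-mounted hi-hat weapon that damages a random targetable enemy in front of the car and is audible only when it has a target.
; TriggerWeapon runs a sphere overlap ahead of the car, filters by Enemy tag and TargetableMessage, then yaws the pivot toward the chosen enemy and sends DamageMessage.
; DrawGunTrace briefly shows an arrow component stretched to the target as a tracer, which Tick keeps aimed while visible.
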(event `SetRotation`
  (`SceneComponent.K2_SetWorldRotation` (`self.Arrow`) (`KismetMathLibrary.FindLookAtRotation` (`SceneComponent.K2_GetComponentLocation` (`self.StaticMesh`)) (`self.TargetGunTracePosition`)) false false :!label _label))

(event `self.ReceiveTick`
  (params (DeltaSeconds :type "Float (single-precision)"))
  (`parent.ReceiveTick` DeltaSeconds)
  (if (`SceneComponent.IsVisible` (`self.Arrow`))
    (goto _label)))

(event `DrawGunTrace`
  (params (TargetPosition :type "Vector Structure") (Distance :type "Float (double-precision)"))
  (bind _arrow (`self.Arrow`))
  (set `self.TargetGunTracePosition` TargetPosition)
  (`self.SetRotation`)
  (set `ArrowComponent.ArrowLength` (/ Distance (`ArrowComponent.ArrowSize` _arrow)) _arrow)
  (`SceneComponent.SetVisibility` _arrow true false)
  (`KismetSystemLibrary.Delay` 0.1)
  (`SceneComponent.SetVisibility` _arrow false false))

(fn `TriggerWeapon`
  (locals (Target :type "Actor Object Reference"))
  (bind _car (`self.Car`))
  (bind _pivot (`self.Pivot`))
  (bind (_returnvalue_roll _returnvalue_pitch) (`KismetMathLibrary.BreakRotator` (`SceneComponent.K2_GetComponentRotation` _pivot)))
  (bind _returnvalue (`self.K2_GetActorLocation` (`local.Target`)))
  (bind (_returnvalue_roll_2 _returnvalue_pitch_2 _returnvalue_yaw) (`KismetMathLibrary.BreakRotator` (`KismetMathLibrary.FindLookAtRotation` (`SceneComponent.K2_GetComponentLocation` (`self.Pivot`)) _returnvalue)))
  (`parent.TriggerWeapon`)
  (bind (_outactors _returnvalue_2) (`KismetSystemLibrary.SphereOverlapActors` (+ (`self.K2_GetActorLocation` _car) (* (`self.GetActorForwardVector` _car) (+ (`self.WeaponRange`) 150.0))) (`self.WeaponRange`) (`|MakeArray` "ObjectTypeQuery3" :!type "EObjectTypeQuery Enum") "/Game/MartinsCoolerContentFolder/BP_EnemyBase.BP_EnemyBase_C" (`|MakeArray` self :!type "Actor Object Reference")))
  (if _returnvalue_2
    (for _array_element _outactors
      (if (`self.ActorHasTag` _array_element "Enemy")
        (bind _targetable (message `/Game/MartinsCoolerContentFolder/I_Targetable.Targetable` _array_element))
        (if (not _targetable)
          (`KismetArrayLibrary.Array_RemoveItem` _outactors _array_element))
        (else
          (`KismetArrayLibrary.Array_RemoveItem` _outactors _array_element))))
    (if (`KismetArrayLibrary.Array_IsEmpty` _outactors)
      (`self.SetInstrumentAudible` false)
      (else
        (set `local.Target` (`KismetArrayLibrary.Array_Random` _outactors))
        (`SceneComponent.K2_SetWorldRotation` _pivot (`KismetMathLibrary.MakeRotator` _returnvalue_roll _returnvalue_pitch _returnvalue_yaw) false false)
        (message `/Game/Game/Pawns/IF_Health.Damage` (`local.Target`) (`self.WeaponDamage`))
        (`self.DrawGunTrace` _returnvalue (`KismetMathLibrary.Vector_Distance` (`SceneComponent.K2_GetComponentLocation` (`self.StaticMesh`)) _returnvalue))
        (`self.SetInstrumentAudible` true)))
    (else
      (`self.SetInstrumentAudible` false))))

(fn `UserConstructionScript`
  (`parent.UserConstructionScript`))