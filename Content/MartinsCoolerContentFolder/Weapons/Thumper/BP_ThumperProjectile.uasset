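; BP_ThumperProjectile is the Thumper weapon's projectile actor, shown here as a self-animating cylinder effect that removes itself.
; On BeginPlay it gives the cylinder a dynamic material instance and plays the Multiplier timeline.
; That one curve drives both the cylinder's flattened, disc-like scale and the material's Opacity, and the actor is destroyed when the timeline finishes.
; The graph contains no movement, collision or damage logic.
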(event `self.ReceiveBeginPlay`
  (bind _returnvalue (`KismetMaterialLibrary.CreateDynamicMaterialInstance` (`PrimitiveComponent.GetMaterial` (`self.Cylinder`) 0)))
  (bind _output_get (set `self.Material` _returnvalue))
  (`PrimitiveComponent.SetMaterial` (`self.Cylinder`) 0 _output_get)
  (bind (_direction _multiplier) (`Timeline|Multiplier` :!via `PlayFromStart`)
    (:`Update`
      (`SceneComponent.SetRelativeScale3D` (`self.Cylinder`) (* _multiplier (0.1 0.1 0.001) 200.0))
      (`MaterialInstanceDynamic.SetScalarParameterValue` (`self.Material`) "Opacity" _multiplier))
    (:`Finished`
      (`self.K2_DestroyActor`))))

(fn `UserConstructionScript`)