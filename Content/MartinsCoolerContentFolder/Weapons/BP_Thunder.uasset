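; Chain-lightning weapon that hits a random targetable enemy within range and toggles its instrument's audibility based on whether it finds one.
; TriggerWeapon damages that target, then ricochets to random enemies near each previous hit, excluding only the current one, so earlier victims can be hit again.
; Beams are arrow components: the main one tracks the stored hit position while visible, and spawned ricochet arrows are destroyed after a brief delay.
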(event `SetRotation`
  (`SceneComponent.K2_SetWorldRotation` (`self.Arrow`) (`KismetMathLibrary.FindLookAtRotation` (`SceneComponent.K2_GetComponentLocation` (`self.StaticMesh`)) (`self.TargetGunTracePosition`)) false false :!label _label))

(event `self.ReceiveTick`
  (params (DeltaSeconds :type "Float (single-precision)"))
  (`parent.ReceiveTick` DeltaSeconds)
  (if (`SceneComponent.IsVisible` (`self.Arrow`))
    (goto _label)))

(event `DrawGunTrace`
  (params (TargetPosition :type "Vector Structure") (Distance :type "Float (double-precision)"))
  (bind _arrows (`self.Arrows`))
  (bind _arrow (`self.Arrow`))
  (set `self.TargetGunTracePosition` TargetPosition)
  (`self.SetRotation`)
  (set `ArrowComponent.ArrowLength` (/ Distance (`ArrowComponent.ArrowSize` _arrow)) _arrow)
  (`SceneComponent.SetVisibility` _arrow true false)
  (`KismetSystemLibrary.Delay` 0.2)
  (`SceneComponent.SetVisibility` _arrow false false)
  (for _array_element _arrows
    (`ActorComponent.K2_DestroyComponent` _array_element))
  (`KismetArrayLibrary.Array_Clear` _arrows))

(fn `SpawnArrow`
  (params (Origin :type "Vector Structure") (Target :type "Vector Structure"))
  (bind _returnvalue (`|AddComponentByClass` "/Script/Engine.ArrowComponent" false (`KismetMathLibrary.MakeTransform` Origin (`KismetMathLibrary.FindLookAtRotation` Origin Target))))
  (`KismetArrayLibrary.Array_Add` (`self.Arrows`) _returnvalue)
  (`SceneComponent.K2_DetachFromComponent` _returnvalue "KeepRelative" "KeepRelative" "KeepRelative" true)
  (`ArrowComponent.SetArrowColor` _returnvalue (struct :`G` 0.879623 :`B` 1.0 :`A` 1.0))
  (set `ArrowComponent.ArrowSize` 4.0 _returnvalue)
  (set `ArrowComponent.ArrowLength` (/ (`KismetMathLibrary.Vector_Distance` Origin Target) 4.0) _returnvalue)
  (`SceneComponent.SetHiddenInGame` _returnvalue false false))

(fn `TriggerWeapon`
  (locals (Target :type "Actor Object Reference") (PreviousTarget :type "Actor Object Reference"))
  (bind _returnvalue (`self.K2_GetActorLocation` (`local.Target`)))
  (`parent.TriggerWeapon`)
  (bind (_outactors _returnvalue_2) (`KismetSystemLibrary.SphereOverlapActors` (`self.K2_GetActorLocation`) (`self.WeaponRange`) (`|MakeArray` "ObjectTypeQuery3" :!type "EObjectTypeQuery Enum") "/Game/MartinsCoolerContentFolder/BP_EnemyBase.BP_EnemyBase_C" (`|MakeArray` self :!type "Actor Object Reference")))
  (if _returnvalue_2
    (for _array_element _outactors
      (if (`self.ActorHasTag` _array_element "Enemy")
        (bind _targetable (message `/Game/MartinsCoolerContentFolder/I_Targetable.Targetable` _array_element))
        (if (not _targetable)
          (`KismetArrayLibrary.Array_RemoveItem` _outactors _array_element))
        (else
          (`KismetArrayLibrary.Array_RemoveItem` _outactors _array_element))))
    (if (`KismetArrayLibrary.Array_IsEmpty` _outactors)
      (`self.SetInstrumentAudible` false)
      (else
        (set `local.Target` (`KismetArrayLibrary.Array_Random` _outactors))
        (message `/Game/Game/Pawns/IF_Health.Damage` (`local.Target`) (`self.WeaponDamage`))
        (`self.DrawGunTrace` _returnvalue (`KismetMathLibrary.Vector_Distance` (`SceneComponent.K2_GetComponentLocation` (`self.StaticMesh`)) _returnvalue))
        (`self.SetInstrumentAudible` true)
        (set `local.PreviousTarget` (`local.Target`))
        (for _ (range 1 (+ (`self.Ricochets`) 1))
          (bind (_outactors_2 _returnvalue_3) (`KismetSystemLibrary.SphereOverlapActors` (`self.K2_GetActorLocation` (`local.PreviousTarget`)) 500.0 (`|MakeArray` "ObjectTypeQuery3" :!type "EObjectTypeQuery Enum") "/Game/MartinsCoolerContentFolder/BP_EnemyBase.BP_EnemyBase_C" (`|MakeArray` self (`local.PreviousTarget`) (`local.Target`) :!type "Actor Object Reference")))
          (if _returnvalue_3
            (for _array_element_2 _outactors_2
              (if (`self.ActorHasTag` _array_element_2 "Enemy")
                (bind _targetable_2 (message `/Game/MartinsCoolerContentFolder/I_Targetable.Targetable` _array_element_2))
                (if (not _targetable_2)
                  (`KismetArrayLibrary.Array_RemoveItem` _outactors_2 _array_element_2))
                (else
                  (`KismetArrayLibrary.Array_RemoveItem` _outactors_2 _array_element_2))))
            (if (not (`KismetArrayLibrary.Array_IsEmpty` _outactors_2))
              (bind _output_get (set `local.Target` (`KismetArrayLibrary.Array_Random` _outactors_2)))
              (`self.SpawnArrow` (`self.K2_GetActorLocation` (`local.PreviousTarget`)) (`self.K2_GetActorLocation` _output_get))
              (message `/Game/Game/Pawns/IF_Health.Damage` (`local.Target`) (`self.WeaponDamage`))
              (set `local.PreviousTarget` (`local.Target`)))))))
    (else
      (`self.SetInstrumentAudible` false))))

(fn `UserConstructionScript`
  (`parent.UserConstructionScript`))