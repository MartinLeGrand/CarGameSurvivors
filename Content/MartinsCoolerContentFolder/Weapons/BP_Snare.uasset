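; BP_Snare is a snare drum weapon that damages the nearest valid enemy in range each time it triggers.
; TriggerWeapon sphere-overlaps for enemies, filters by tag and targetable state, then yaws the snare toward the closest and sends it damage.
; An arrow component doubles as a brief gun trace, stretched to the target and re-aimed on Tick while visible.
; The instrument is audible only when a target is found.
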(event `SetRotation`
  (`SceneComponent.K2_SetWorldRotation` (`self.Arrow`) (`KismetMathLibrary.FindLookAtRotation` (`self.K2_GetActorLocation`) (`self.TargetGunTracePosition`)) false false :!label _label))

(event `self.ReceiveTick`
  (params (DeltaSeconds :type "Float (single-precision)"))
  (`parent.ReceiveTick` DeltaSeconds)
  (if (`SceneComponent.IsVisible` (`self.Arrow`))
    (goto _label)))

(event `DrawGunTrace`
  (params (TargetPosition :type "Vector Structure") (Distance :type "Float (double-precision)"))
  (bind _arrow (`self.Arrow`))
  (set `self.TargetGunTracePosition` TargetPosition)
  (`self.SetRotation`)
  (set `ArrowComponent.ArrowLength` (/ Distance (`ArrowComponent.ArrowSize` _arrow)) _arrow)
  (`SceneComponent.SetVisibility` _arrow true false)
  (`KismetSystemLibrary.Delay` 0.1)
  (`SceneComponent.SetVisibility` _arrow false false))

(fn `TriggerWeapon`
  (locals (Target :type "Actor Object Reference"))
  (bind _returnvalue (`self.K2_GetActorLocation`))
  (bind _snare (`self.Snare`))
  (bind (_returnvalue_roll _returnvalue_pitch) (`KismetMathLibrary.BreakRotator` (`SceneComponent.K2_GetComponentRotation` _snare)))
  (bind _returnvalue_2 (`self.K2_GetActorLocation` (`local.Target`)))
  (bind (_returnvalue_roll_2 _returnvalue_pitch_2 _returnvalue_yaw) (`KismetMathLibrary.BreakRotator` (`KismetMathLibrary.FindLookAtRotation` _returnvalue _returnvalue_2)))
  (`parent.TriggerWeapon`)
  (bind (_outactors _returnvalue_3) (`KismetSystemLibrary.SphereOverlapActors` (`self.K2_GetActorLocation`) (`self.WeaponRange`) (`|MakeArray` "ObjectTypeQuery3" :!type "EObjectTypeQuery Enum") "/Game/MartinsCoolerContentFolder/BP_EnemyBase.BP_EnemyBase_C" (`|MakeArray` self :!type "Actor Object Reference")))
  (if _returnvalue_3
    (for _array_element _outactors
      (if (`self.ActorHasTag` _array_element "Enemy")
        (bind _targetable (message `/Game/MartinsCoolerContentFolder/I_Targetable.Targetable` _array_element))
        (if (not _targetable)
          (`KismetArrayLibrary.Array_RemoveItem` _outactors _array_element))
        (else
          (`KismetArrayLibrary.Array_RemoveItem` _outactors _array_element))))
    (if (`KismetArrayLibrary.Array_IsEmpty` _outactors)
      (`self.SetInstrumentAudible` false)
      (else
        (set `local.Target` (`.ReturnValue` (`GameplayStatics.FindNearestActor` (`self.K2_GetActorLocation`) _outactors)))
        (`SceneComponent.K2_SetWorldRotation` _snare (`KismetMathLibrary.MakeRotator` _returnvalue_roll _returnvalue_pitch _returnvalue_yaw) false false)
        (message `/Game/Game/Pawns/IF_Health.Damage` (`local.Target`) (`self.WeaponDamage`))
        (`self.DrawGunTrace` _returnvalue_2 (`KismetMathLibrary.Vector_Distance` _returnvalue _returnvalue_2))
        (`self.SetInstrumentAudible` true)))
    (else
      (`self.SetInstrumentAudible` false))))

(fn `UserConstructionScript`
  (`parent.UserConstructionScript`))