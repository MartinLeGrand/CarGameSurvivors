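; BP_WeaponParent is a base weapon that fires in sync with music markers, with TriggerWeapon left empty for child Blueprints.
; One tick after BeginPlay it binds to the Beat Manager's beat marker event and triggers when the marker name matches MarkerToRespondTo.
; SetInstrumentAudible switches the weapon's instrument on or off through a named parameter on the manager's FMOD audio.
; The health getters are stubs returning zero.
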(event `self.ReceiveBeginPlay`
  (`KismetSystemLibrary.DelayUntilNextTick`)
  (add `/Game/MartinsCoolerContentFolder/BP_BeatManager.BeatMarker` (`/Game/Game/GameModes/Getters.Get Beat Manager`) (delegate `BeatMarker_Event`)))

(event `BeatMarker_Event`
  (params (MarkerName :type String))
  (if (`KismetStringLibrary.EqualEqual_StrStr` MarkerName (`self.MarkerToRespondTo`))
    (`self.TriggerWeapon`)))

(fn `Get Current Health`
  (returns (ReturnValue :type Integer))
  (return 0))

(fn `Get Current Health Percent`
  (returns (ReturnValue :type "Float (double-precision)"))
  (return 0.0))

(fn `SetInstrumentAudible`
  (params (Audible :type Boolean))
  (`FMODAudioComponent.SetParameter` (`/Game/MartinsCoolerContentFolder/BP_BeatManager.FMODAudio` (`/Game/Game/GameModes/Getters.Get Beat Manager`)) (`KismetStringLibrary.Conv_StringToName` (`self.ParameterToMute`)) (`KismetMathLibrary.SelectFloat` 1.0 0.0 Audible)))

(fn `TriggerWeapon`)

(fn `UserConstructionScript`)