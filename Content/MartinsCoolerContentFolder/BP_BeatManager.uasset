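; Beat manager actor that relays FMOD timeline markers through a BeatMarker dispatcher to sync gameplay with the music.
; On BeginPlay it also spawns the enemy spawner actor and starts a looping timer that counts enemies, prints the total and feeds it, normalized, into an FMOD parameter.
; SpawnAndAttachWeapon maps a weapon type to its class, spawns it at its default transform, attaches it to the player car and records the class.
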(event `self.ReceiveBeginPlay`
  (add `FMODAudioComponent.OnTimelineMarker` (`self.FMODAudio`) (delegate `OnTimelineMarker_Event`))
  (`KismetSystemLibrary.K2_SetTimerDelegate` (delegate `EnemyCounting`) 1.0 true)
  (`|SpawnActorFromClass` "/Game/MartinsCoolerContentFolder/BP_EnemySpawnerSpawner.BP_EnemySpawnerSpawner_C" (`KismetMathLibrary.MakeTransform` (0.0 0.0 0.0)) "Undefined" "MultiplyWithRoot" null null))

(event `OnTimelineMarker_Event`
  (params (Name :type String) (Position :type Integer))
  (`self.BeatMarker` Name))

(event `EnemyCounting`
  (bind _outactors (`GameplayStatics.GetAllActorsOfClass` "/Game/MartinsCoolerContentFolder/BP_EnemyBase.BP_EnemyBase_C"))
  (bind _returnvalue (`KismetArrayLibrary.Array_Length` _outactors))
  (`KismetSystemLibrary.PrintString` (`KismetStringLibrary.Conv_IntToString` _returnvalue))
  (`FMODAudioComponent.SetParameter` (`self.FMODAudio`) "amountOfEnemies" (`KismetMathLibrary.MapRangeClamped` (`KismetMathLibrary.Conv_IntToDouble` _returnvalue) 0.0 200.0 0.0 1.0)))

(event `SpawnAndAttachWeapon`
  (params (Weapon :type "/Game/MartinsCoolerContentFolder/E_Weapons Enum" :default "NewEnumerator0") (Player :type "/Game/Game/Pawns/Car/P_Car Object Reference"))
  (bind _returnvalue (select `/Game/MartinsCoolerContentFolder/E_Weapons` Weapon :`NewEnumerator0` "/Game/MartinsCoolerContentFolder/Weapons/BP_Snare.BP_Snare_C" :`NewEnumerator1` "/Game/MartinsCoolerContentFolder/Weapons/BP_Thumper.BP_Thumper_C" :`NewEnumerator2` "/Game/MartinsCoolerContentFolder/Weapons/BP_HiHat.BP_HiHat_C" :`NewEnumerator3` "/Game/MartinsCoolerContentFolder/Weapons/BP_GrenadeLauncher.BP_GrenadeLauncher_C" :`NewEnumerator4` "/Game/MartinsCoolerContentFolder/Weapons/BP_Thunder.BP_Thunder_C" :`NewEnumerator5` "/Game/MartinsCoolerContentFolder/Weapons/BP_RocketLauncher.BP_RocketLauncher_C" :!type "/Game/MartinsCoolerContentFolder/Weapons/BP_WeaponParent Class Reference"))
  (bind _returnvalue_2 (`|SpawnActorFromClass` _returnvalue (defaults `Object` _returnvalue) "Undefined" "MultiplyWithRoot" Player Player null))
  (`self.K2_AttachToActor` _returnvalue_2 Player "None" "KeepRelative" "KeepRelative" "KeepRelative" true)
  (`KismetArrayLibrary.Array_Add` (`/Game/Game/Pawns/Car/P_Car.Weapons` Player) _returnvalue))

(fn `UserConstructionScript`)