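; BP_EnemySpawner is a placed actor that periodically spawns random enemies around itself, scaled to the player's level, with a bobbing arrow.
; XP manager level-ups rebuild a weighted spawn pool from that level's wave map, repeating classes by key, and restart a looping, randomly staggered timer.
; Each tick of that timer spawns a per-level count at randomized horizontal offsets, skipping the wave when framerate drops below 30 FPS.
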(event `self.ReceiveBeginPlay`
  (`|ExecutionSequence`
    (:`then_0`
      (set `self.Relative Location` (`SceneComponent.RelativeLocation` (`self.Arrow`)))
      (bind (_direction _multiplier) (`Timeline|Timeline` :!label _label)
        (:`Update`
          (`SceneComponent.K2_SetRelativeLocation` (`self.Arrow`) (+ (`self.Relative Location`) (`KismetMathLibrary.MakeVector` 0.0 0.0 (* _multiplier 100.0))) false false))
        (:`Finished`
          (goto _label :!via `PlayFromStart`))))
    (:`then_1`
      (add `/Game/Game/GameModes/BP_XpManager.Leveled Up` (`/Game/Game/GameModes/Getters.Get XP Manager`) (delegate `Leveled Up_Event`))
      (`self.Leveled Up_Event` 0 1))))

(event `SetSpawnTimer`
  (bind _output (`|GetArrayItem` (`self.TimeBetweenSpawnEvents`) (`self.CurrentLevel`)))
  (`KismetSystemLibrary.K2_ClearAndInvalidateTimerHandle` (`self.Timer`))
  (bind _returnvalue (`KismetSystemLibrary.K2_SetTimerDelegate` (delegate `SpawnEnemy`) _output true false (`KismetMathLibrary.RandomFloatInRange` 0.0 _output)))
  (set `self.Timer` _returnvalue))

(event `Leveled Up_Event`
  (params (`Previous Level` :type Integer) (`New Level` :type Integer))
  (bind _output_get (set `self.CurrentLevel` `New Level`))
  (`KismetArrayLibrary.Array_Clear` (`self.SpawnArray`))
  (bind (_keypin _valuepin) (`|MapForEach` (select `int` _output_get :`0` _ :`1` (`self.Wave1`) :`2` (`self.Wave2`) :`3` (`self.Wave3`) :`4` (`self.Wave4`) :`5` (`self.Wave5`) :`6` (`self.Wave6`) :`7` (`self.Wave7`) :`8` (`self.Wave8`) :`9` (`self.Wave9`) :`10` (`self.Wave10`)))
    (:`then`
      (for _ (range 1 (+ _keypin 1))
        (`KismetArrayLibrary.Array_Add` (`self.SpawnArray`) _valuepin)))
    (:`CompletedPin`
      (`self.SetSpawnTimer`))))

(event `SpawnEnemy`
  (bind _spawnlocationvariance (`self.SpawnLocationVariance`))
  (bind _returnvalue (`KismetMathLibrary.RandomFloatInRange` (* _spawnlocationvariance -1.0) _spawnlocationvariance))
  (if (< (/ 1.0 (`GameplayStatics.GetWorldDeltaSeconds`)) 30.0)
    (`KismetSystemLibrary.PrintString` "Too much lag, skipped spawn wave" true true (struct :`R` 1.0 :`A` 1.0) 5.0 "lagwarning")
    (else
      (for _ (range 1 (+ (`|GetArrayItem` (`self.UnitsToSpawn`) (`self.CurrentLevel`)) 1))
        (`|SpawnActorFromClass` (`KismetArrayLibrary.Array_Random` (`self.SpawnArray`)) (`KismetMathLibrary.MakeTransform` (+ (`SceneComponent.K2_GetComponentLocation` (`self.Scene`)) (`KismetMathLibrary.MakeVector` _returnvalue _returnvalue))) "Undefined" "MultiplyWithRoot" null null)))))

(fn `UserConstructionScript`)